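; BP_PlaneteSolaire is a solar-system planet actor that assigns planet materials and attempts to draw movement lines.
; After a short delay on BeginPlay, each instance loops over all planets, setting their mesh materials from an array by index.
; Every Tick, it loops over all planets, calling 2D DrawLine from its stored previous position to theirs, then storing its own location.
; A Niagara particle spawn is present but unconnected.
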(event `self.ReceiveBeginPlay`
  (`KismetSystemLibrary.Delay` 0.5)
  (bind _outactors (`GameplayStatics.GetAllActorsOfClass` "BP_PlaneteSolaire_C"))
  (for (_array_element _array_index) _outactors
    (`PrimitiveComponent.SetMaterial` (`CelestialBody.StaticMeshComponent` _array_element) 0 (`|GetArrayItem` (`self.material`) _array_index))))

(event `self.ReceiveTick`
  (params (DeltaSeconds :type "Float (single-precision)"))
  (bind _outactors (`GameplayStatics.GetAllActorsOfClass` "BP_PlaneteSolaire_C"))
  (for _array_element _outactors
    (if (not (== (`self.Encienne position`) (0.0 0.0 0.0)))
      (`WidgetBlueprintLibrary.DrawLine` (struct) (`KismetMathLibrary.Conv_VectorToVector2D` (`self.Encienne position`)) (`KismetMathLibrary.Conv_VectorToVector2D` (`self.K2_GetActorLocation` _array_element))))
    (set `self.Encienne position` (`self.K2_GetActorLocation`))))

(fn `UserConstructionScript`)