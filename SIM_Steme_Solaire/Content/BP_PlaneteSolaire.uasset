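; BP_PlaneteSolaire is a solar planet actor that sets planet materials and spawns an effect at its position.
; Shortly after BeginPlay, each instance gathers every BP_PlaneteSolaire and assigns each mesh the Material array entry matching its index in that list.
; Tick calls SpawnSystemAtLocation at the actor's location every frame, with no system asset specified in the call.
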(event `self.ReceiveBeginPlay`
  (`KismetSystemLibrary.Delay` 0.5)
  (bind _outactors (`GameplayStatics.GetAllActorsOfClass` "BP_PlaneteSolaire_C"))
  (for (_array_element _array_index) _outactors
    (`PrimitiveComponent.SetMaterial` (`CelestialBody.StaticMeshComponent` _array_element) 0 (`|GetArrayItem` (`self.material`) _array_index))))

(event `self.ReceiveTick`
  (params (DeltaSeconds :type "Float (single-precision)"))
  (`NiagaraFunctionLibrary.SpawnSystemAtLocation` null (`self.K2_GetActorLocation` self)))

(fn `UserConstructionScript`)