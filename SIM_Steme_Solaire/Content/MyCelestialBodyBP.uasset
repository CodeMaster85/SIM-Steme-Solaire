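; Celestial body Blueprint that procedurally generates a planet's look in its Construction Script from the seeded stream Graine.
; When the B_creationObjet widget's seed message is empty, it reseeds Graine randomly, then sets the planet material's terrain and color parameters and the actor scale.
; About half the planets show a tilted ring plane with its own randomized dynamic material.
; A non-empty message only sets Graine, skipping generation.
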(event `/Game/b_PauseJouer.PauseJouer`
  (params (PauseJouer :type Boolean)))

(fn `getgraine`)

(fn `tableauBruit`)

(fn `UserConstructionScript`
  (locals (vide :type Text))
  (bind _manneau (`self.MAnneau`))
  (bind _manneau_2 (`self.MAnneau`))
  (bind _graine (`self.graine`))
  (bind _mplanete (`self.MPlanete`))
  (bind _plane (`self.Plane`))
  (bind _graine_2 (`self.graine`))
  (bind _returnvalue (`KismetMathLibrary.RandomFloatInRangeFromStream` _graine 0.0 1.0))
  (bind _foundwidgets (`WidgetBlueprintLibrary.GetAllWidgetsOfClass` "/Game/UI/b_creationObjet.b_creationObjet_C"))
  (bind _graine_3 (message `/Game/celestialbodyVersConst.getgraine` _foundwidgets))
  ;[1 1 1] texture aléatoire de la planète
  ;;[1 1 1] génération de la seed pour la planète
  (bind _returnvalue_2 (`KismetMaterialLibrary.CreateDynamicMaterialInstance` "/Game/M_generation.M_generation"))
  (if (`KismetTextLibrary.EqualEqual_TextText` _graine_3 (`local.vide`))
    (`KismetMathLibrary.SeedRandomStream` (`self.graine`))
    ;;[1 1 1] rapport eau terre entre 0 et 1
    (bind _output_get (set `self.MPlanete` _returnvalue_2))
    (`MaterialInstanceDynamic.SetScalarParameterValue` _output_get "RapportEauTerre" (`KismetMathLibrary.RandomFloatInRangeFromStream` _graine 0.0 2.0))
    (`MaterialInstanceDynamic.SetScalarParameterValue` _output_get "EauOuLave" (`KismetMathLibrary.RandomFloatInRangeFromStream` _graine 0.0 1.0))
    (`MaterialInstanceDynamic.SetScalarParameterValue` _output_get "couleurSol" (`KismetMathLibrary.RandomFloatInRangeFromStream` _graine 0.0 1.0))
    ;;[1 1 1] détermine les couleurs aléatoirement
    (`MaterialInstanceDynamic.SetVectorParameterValue` _mplanete "lave" (`KismetMathLibrary.Conv_VectorToLinearColor` (`KismetMathLibrary.Normal` (`KismetMathLibrary.MakeVector` (`KismetMathLibrary.RandomFloatInRangeFromStream` _graine 0.0 1.0) 0.1))))
    (`MaterialInstanceDynamic.SetVectorParameterValue` _mplanete "eau" (`KismetMathLibrary.Conv_VectorToLinearColor` (`KismetMathLibrary.Normal` (`KismetMathLibrary.MakeVector` 0.5 0.0 0.5))))
    (`MaterialInstanceDynamic.SetVectorParameterValue` _mplanete "mauve" (`KismetMathLibrary.Conv_VectorToLinearColor` (`KismetMathLibrary.Normal` (`KismetMathLibrary.MakeVector` 0.0 _returnvalue 1.0))))
    (`MaterialInstanceDynamic.SetVectorParameterValue` _mplanete "brun" (`KismetMathLibrary.Conv_VectorToLinearColor` (`KismetMathLibrary.Normal` (`KismetMathLibrary.MakeVector` 1.0 _returnvalue))))
    (`self.SetActorScale3D` (`KismetMathLibrary.Conv_DoubleToVector` (`KismetMathLibrary.RandomFloatInRangeFromStream` _graine 0.5 5.0)))
    (`PrimitiveComponent.SetMaterial` (`self.StaticMeshComponent`) 0 (`self.MPlanete`))
    (if (< (`KismetMathLibrary.RandomFloatInRangeFromStream` _graine 0.0 1.0) 0.5)
      ;[1 1 1] On affiche l'anneau et on lui ajoute une rotation random
      (`SceneComponent.SetVisibility` _plane true false)
      (`SceneComponent.K2_SetWorldRotation` _plane (`KismetMathLibrary.MakeRotator` 0.0 (`KismetMathLibrary.RandomFloatInRangeFromStream` _graine 0.0 180.0)) false false)
      ;[1 1 1] génération de l'anneau
      (bind _returnvalue_3 (`KismetMaterialLibrary.CreateDynamicMaterialInstance` "/Game/m_GenerationAnneau.m_GenerationAnneau"))
      (set `self.MAnneau` _returnvalue_3)
      (`MaterialInstanceDynamic.SetVectorParameterValue` _manneau "1" (`KismetMathLibrary.Conv_VectorToLinearColor` (`KismetMathLibrary.Normal` (`KismetMathLibrary.MakeVector` 1.0 0.0 (`KismetMathLibrary.RandomFloatInRangeFromStream` _graine_2 0.0 1.0)))))
      (`MaterialInstanceDynamic.SetVectorParameterValue` _manneau "2" (`KismetMathLibrary.Conv_VectorToLinearColor` (`KismetMathLibrary.Normal` (`KismetMathLibrary.MakeVector` 0.0 (`KismetMathLibrary.RandomFloatInRangeFromStream` _graine_2 0.0 1.0) 1.0))))
      (`MaterialInstanceDynamic.SetVectorParameterValue` _manneau "3" (`KismetMathLibrary.Conv_VectorToLinearColor` (`KismetMathLibrary.Normal` (`KismetMathLibrary.MakeVector` (`KismetMathLibrary.RandomFloatInRangeFromStream` _graine_2 0.0 1.0) 1.0 1.0))))
      (`MaterialInstanceDynamic.SetVectorParameterValue` _manneau "4" (`KismetMathLibrary.Conv_VectorToLinearColor` (`KismetMathLibrary.Normal` (`KismetMathLibrary.MakeVector` 1.0 (`KismetMathLibrary.RandomFloatInRangeFromStream` _graine_2 0.0 1.0) 0.4))))
      (`MaterialInstanceDynamic.SetScalarParameterValue` _manneau_2 "intérieur" (`KismetMathLibrary.RandomFloatInRangeFromStream` _graine_2 0.2 0.4))
      (`MaterialInstanceDynamic.SetScalarParameterValue` _manneau_2 "extérieur" (`KismetMathLibrary.RandomFloatInRangeFromStream` _graine_2 0.4 0.7))
      (`MaterialInstanceDynamic.SetScalarParameterValue` _manneau_2 "dureté" (`KismetMathLibrary.RandomFloatInRangeFromStream` _graine_2 0.0 1.0))
      (`MaterialInstanceDynamic.SetScalarParameterValue` _manneau_2 "nbDeCercle" (`KismetMathLibrary.RandomFloatInRangeFromStream` _graine_2 1.0 10.0))
      (`MaterialInstanceDynamic.SetScalarParameterValue` _manneau_2 "controle" (`KismetMathLibrary.RandomFloatInRangeFromStream` _graine_2 0.0 1.0))
      (`PrimitiveComponent.SetMaterial` (`self.Plane`) 0 (`self.MAnneau`)))
    (else
      (set `self.graine` (`KismetMathLibrary.MakeRandomStream` (`KismetStringLibrary.Conv_StringToInt` (`KismetTextLibrary.Conv_TextToString` _graine_3)))))))